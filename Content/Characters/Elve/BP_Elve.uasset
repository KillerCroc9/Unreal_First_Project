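; BP_Elve is an elf character Blueprint that handles basic player movement and mouse look.
; Forward/backward and right/left axis inputs add movement along the forward and right vectors of the control rotation.
; Mouse axes drive controller pitch and yaw, so look direction steers movement.
; Forward movement uses the full control rotation rather than yaw alone, and the construction script is empty.
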(event Input|AxisEvents|InputAxisMoveForward/Backward
  (params (AxisValue :type Float%20%28single-precision%29))
  ;[0 0 0] Movement
  (Pawn|Input|AddMovementInput (Math|Vector|GetForwardVector (Pawn|GetControlRotation :!class /Script/Engine.Pawn)) AxisValue false))

(event Input|AxisEvents|InputAxisMoveRight/Left
  (params (AxisValue :type Float%20%28single-precision%29))
  ;[0 0 0] Movement
  (Pawn|Input|AddMovementInput (Math|Vector|GetRightVector (Pawn|GetControlRotation :!class /Script/Engine.Pawn)) AxisValue false))

(event Input|AxisEvents|InputAxisLookUp/DownMouse
  (params (AxisValue :type Float%20%28single-precision%29))
  ;[0 0 0] Camera
  (Pawn|Input|AddControllerPitchInput AxisValue))

(event Input|AxisEvents|InputAxisTurnRight/LeftMouse
  (params (AxisValue :type Float%20%28single-precision%29))
  ;[0 0 0] Camera
  (Pawn|Input|AddControllerYawInput AxisValue))

(fn ConstructionScript)